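; AI slime enemy that chases and attacks the player and dies when damage brings its health to exactly zero.
; On PawnSensing sight it compares player and first SpiritOrbOG distances, chasing a nearer KnightOfLight and widening sight; the orb-chase call is unwired.
; A delayed Tick applies close-range damage, with a looping counter as cooldown.
; The player range check spawns a slime trail when out of range; Roaming and Patrol calls never run.
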(event OnSeePawn(PawnSensing)
  (params (Pawn :type Pawn%20Object%20Reference))
  ;[1 1 1] Chase Player When Seen
  (CallFunction|CheckPlayerRange)
  (CallFunction|CheckSpiritOrbRange)
  (if (or (Variables|Default|GetSpiritOrbInRange) (Variables|Default|GetPlayerInRange))
    (Development|PrintString "Made it past branch")
    (Math|Float|CompareFloat (Variables|Default|GetPlayerDistance) (Variables|Default|GetSpiritOrbDistance)
      (:>
        (bind _outactors (Actor|GetAllActorsOfClass "/Game/bluePrints/spiritOrbOG.spiritOrbOG_C" :!label _label)))
      (:==
        (goto _label))
      (:<
        (bind _asknight_of_light (Utilities|Casting|CastToKnightOfLight Pawn))
        (CallFunction|ChasePlayer _asknight_of_light)
        (Variables|/Script/AIModule.PawnSensingComponent|SetSightRadius (Variables|Default|GetPawnSensing) 7e+03)))))

(event Custom|CheckPlayerRange
  (bind _returnvalue (Game|GetPlayerCharacter 0))
  (bind _returnvalue_2 (Transformation|GetDistanceTo _returnvalue))
  (if (<= _returnvalue_2 (Variables|Default|GetAttackRange))
    (Variables|Default|SetPlayerInRange true)
    (Variables|Default|SetPlayerDistance _returnvalue_2)
    (else
      (Variables|Default|SetPlayerInRange false)
      (Effects|SpawnEmitteratLocation "/Game/customArt/Enemies/Slime_trail.Slime_trail" (+ (Transformation|GetActorLocation) "0,-10.000000,0.000000")))))

(event Custom|CheckSpiritOrbRange
  (bind _outactors (Actor|GetAllActorsOfClass "/Game/bluePrints/spiritOrbOG.spiritOrbOG_C"))
  (if (<= (Transformation|GetDistanceTo (Utilities|Array|Get(acopy) _outactors)) (Variables|Default|GetAttackRange))
    (Variables|Default|SetSpiritOrbInRange true)
    (Variables|Default|SetSpiritOrbDistance (Transformation|GetDistanceTo (Utilities|Array|Get(acopy) _outactors)))
    (else
      (Variables|Default|SetSpiritOrbInRange false))))

(event Custom|ChasePlayer
  (params (ActorToChase :type Actor%20Object%20Reference))
  ;[1 1 1] AI Chase Player
  (AI|AIMoveTo self "0, 0, 0" ActorToChase 5.0 false))

(event Custom|AttackDelaySet
  ;[1 1 1] Reset Attack Delay
  (while (< (Variables|Default|GetAttackDelay) 6.0)
    (Math|Float|IncrementFloat (Variables|Default|GetAttackDelay)
      (:%20%20
        (Utilities|FlowControl|Delay 1.0))))
  (Variables|Default|SetAttack? true)
  (Variables|Default|SetAttackDelay 0.0))

(event EventBeginPlay
  ;[1 1 1] Begin AI Functions
  (switch Utilities|FlowControl|Switch|SwitchonAI_State (Variables|Default|GetAIState)
    (:NewEnumerator2
      (CallFunction|ChasePlayer))))

(event Game|Damage|EventAnyDamage
  (params (Damage :type Float%20%28single-precision%29) (DamageType :type Damage%20Type%20Object%20Reference) (InstigatedBy :type Controller%20Object%20Reference) (DamageCauser :type Actor%20Object%20Reference))
  ;[1 1 1] Take Damage and Check for Death
  (Variables|Default|SetHealth (- (Variables|Default|GetHealth) Damage))
  (if (== (Variables|Default|GetHealth) 0.0)
    (Actor|DestroyActor)))

(event EventTick
  (params (DeltaSeconds :type Float%20%28single-precision%29))
  (bind _returnvalue (Game|GetPlayerCharacter 0))
  ;[1 1 1] Attack
  (Utilities|FlowControl|Delay 1.0)
  (if (Variables|Default|GetAttack?)
    (if (< (Transformation|GetDistanceTo _returnvalue) 1.5e+02)
      (Game|Damage|ApplyDamage _returnvalue (Variables|Default|GetDamage) 0 0)
      (Variables|Default|SetAttack? false)
      (CallFunction|AttackDelaySet))))

(fn ConstructionScript)