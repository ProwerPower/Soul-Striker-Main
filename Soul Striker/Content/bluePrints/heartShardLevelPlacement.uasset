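; Heart shard pickup placed in levels that adds one to the KnightOfLight's health shard count.
; A looping timer started on BeginPlay spins the HeartShard in yaw and bobs it vertically, reversing direction at fixed world-space Z limits.
; Overlapping the Box with a KnightOfLight increments CurrentHealthShards and destroys the actor; other actors are ignored.
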(event OnComponentBeginOverlap(Box)
  (params (OverlappedComponent :type Primitive%20Component%20Object%20Reference) (OtherActor :type Actor%20Object%20Reference) (OtherComp :type Primitive%20Component%20Object%20Reference) (OtherBodyIndex :type Integer) (bFromSweep :type Boolean) (SweepResult :type Hit%20Result%20Structure%20%28by%20ref%29))
  (bind _asknight_of_light (Utilities|Casting|CastToKnightOfLight OtherActor))
  (Variables|/Game/ThirdPersonBP/Blueprints/KnightOfLight.KnightOfLight_C|SetcurrentHealthShards _asknight_of_light (+ (Variables|/Game/ThirdPersonBP/Blueprints/KnightOfLight.KnightOfLight_C|GetcurrentHealthShards _asknight_of_light) 1))
  (Actor|DestroyActor))

(event EventBeginPlay
  (Utilities|Time|SetTimerbyFunctionName 0 "bobAndRotateShard" 0.1 true))

(fn ConstructionScript)

(fn BobandRotateShard
  (bind _heartshard (Variables|Default|GetheartShard))
  (bind _heartshard_2 (Variables|Default|GetheartShard))
  (bind _returnvalue (Transformation|GetWorldRotation _heartshard))
  (bind _returnvalue_2 (Transformation|GetWorldLocation _heartshard_2))
  (Transformation|SetWorldRotation _heartshard (Math|Rotator|MakeRotator (.roll _returnvalue) (.pitch _returnvalue) (+ (.yaw _returnvalue) 1.0)) false false)
  (if (<= (.z _returnvalue_2) (Variables|Default|GetkeyMinFloat))
    (bind _output_get (Variables|Default|SetkeyFloatMagicValue (* (Variables|Default|GetkeyFloatMagicValue) -1.0)))
    (Transformation|SetWorldLocation (Variables|Default|GetheartShard) (Math|Vector|MakeVector (.x _returnvalue_2) (.y _returnvalue_2) (+ (.z _returnvalue_2) _output_get)) false false)
    (elif (>= (.z _returnvalue_2) (Variables|Default|GetkeyMaxFloat))
      (bind _output_get_2 (Variables|Default|SetkeyFloatMagicValue (* (Variables|Default|GetkeyFloatMagicValue) -1.0)))
      (Transformation|SetWorldLocation (Variables|Default|GetheartShard) (Math|Vector|MakeVector (.x _returnvalue_2) (.y _returnvalue_2) (+ (.z _returnvalue_2) _output_get_2)) false false)
      (else
        (Transformation|SetWorldLocation (Variables|Default|GetheartShard) (Math|Vector|MakeVector (.x _returnvalue_2) (.y _returnvalue_2) (+ (.z _returnvalue_2) (Variables|Default|GetkeyFloatMagicValue))) false false)))))