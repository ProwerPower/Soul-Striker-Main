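; Checkpoint actor that passes a respawn location to the KnightOfLight player and raises a DMC-style door.
; A looping timer started on BeginPlay polls overlapping actors instead of using overlap events.
; While the knight overlaps, each tick sends the stored X/Y/Z coordinates through RespawnAtPrevLocation.
; It then makes the first DMC_DORS actor's mesh visible and sets its collision to physics-only.
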(event EventBeginPlay
  (Utilities|Time|SetTimerbyFunctionName 0 "checkForPlayerAndSetRespawnPoint" 0.1 true))

(fn ConstructionScript)

(fn CheckforPlayerandSetRespawnPoint
  (bind _asknight_of_light (Utilities|Casting|CastToKnightOfLight (Utilities|Array|Get(acopy) (Collision|GetOverlappingActors "/Game/ThirdPersonBP/Blueprints/KnightOfLight.KnightOfLight_C" :!class /Script/Engine.Actor))))
  (Default|RespawnatPrevLocation _asknight_of_light (Variables|Default|GetxRespawnLoc) (Variables|Default|GetyRespawnLoc) (Variables|Default|GetzRespawnLoc))
  (bind _outactors (Actor|GetAllActorsOfClass "/Game/bluePrints/DMC_DORS.DMC_DORS_C"))
  (Rendering|SetVisibility (Variables|/Script/Engine.StaticMeshActor|GetStaticMeshComponent (Utilities|Array|Get(acopy) _outactors)) true false)
  (Collision|SetCollisionEnabled (Variables|/Script/Engine.StaticMeshActor|GetStaticMeshComponent (Utilities|Array|Get(acopy) _outactors)) "PhysicsOnly"))