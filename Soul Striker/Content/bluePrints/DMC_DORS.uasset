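; DMC_DORS is a trigger-driven barrier, likely a door, that appears behind the KnightOfLight and bounces spirit orbs.
; While HasBeenTriggered is false, the knight leaving the Box makes the static mesh visible and collidable.
; While it is true, an entering spiritOrbOG stores its X/Y physics velocity, then runs BallBounceNonDestructible on exit.
; This graph only reads HasBeenTriggered and never sets it.
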(event OnComponentBeginOverlap(Box)
  (params (OverlappedComponent :type Primitive%20Component%20Object%20Reference) (OtherActor :type Actor%20Object%20Reference) (OtherComp :type Primitive%20Component%20Object%20Reference) (OtherBodyIndex :type Integer) (bFromSweep :type Boolean) (SweepResult :type Hit%20Result%20Structure%20%28by%20ref%29))
  (if (Variables|Default|GetHasBeenTriggered)
    (bind _asspirit_orb_og (Utilities|Casting|CastTospiritOrbOG OtherActor))
    (bind _returnvalue (Physics|GetPhysicsLinearVelocity (Variables|/Game/bluePrints/spiritOrbOG.spiritOrbOG_C|GetSphere _asspirit_orb_og) "None"))
    (Variables|/Game/bluePrints/spiritOrbOG.spiritOrbOG_C|SetOriginal%20Velocity%20X _asspirit_orb_og (.x _returnvalue))
    (Variables|/Game/bluePrints/spiritOrbOG.spiritOrbOG_C|SetOriginal%20Velocity%20Y _asspirit_orb_og (.y _returnvalue))))

(event OnComponentEndOverlap(Box)
  (params (OverlappedComponent :type Primitive%20Component%20Object%20Reference) (OtherActor :type Actor%20Object%20Reference) (OtherComp :type Primitive%20Component%20Object%20Reference) (OtherBodyIndex :type Integer))
  (if (Variables|Default|GetHasBeenTriggered)
    (bind _asspirit_orb_og (Utilities|Casting|CastTospiritOrbOG OtherActor))
    (Default|BallBounceNon-Destructible _asspirit_orb_og)
    (else
      (Utilities|Casting|CastToKnightOfLight OtherActor)
      (Rendering|SetVisibility (Variables|Debug|GetStaticMeshComponent) true false)
      (Collision|SetCollisionEnabled (Variables|Debug|GetStaticMeshComponent) "QueryAndPhysics"))))

(fn ConstructionScript)