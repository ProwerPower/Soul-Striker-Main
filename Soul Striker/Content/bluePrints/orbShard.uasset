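; Orb shard pickup that a KnightOfLight character collects to raise its CurrentOrbShards count.
; On BeginPlay, a randomized velocity-change impulse pops the shard upward with some horizontal scatter.
; Overlapping its Box with the knight increments the count and destroys the shard.
; A ShardFloat function nudges world rotation on all three axes, but the event graph never calls it.
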(event OnComponentBeginOverlap(Box)
  (params (OverlappedComponent :type Primitive%20Component%20Object%20Reference) (OtherActor :type Actor%20Object%20Reference) (OtherComp :type Primitive%20Component%20Object%20Reference) (OtherBodyIndex :type Integer) (bFromSweep :type Boolean) (SweepResult :type Hit%20Result%20Structure%20%28by%20ref%29))
  (bind _asknight_of_light (Utilities|Casting|CastToKnightOfLight OtherActor))
  (Variables|/Game/ThirdPersonBP/Blueprints/KnightOfLight.KnightOfLight_C|SetcurrentOrbShards _asknight_of_light (+ (Variables|/Game/ThirdPersonBP/Blueprints/KnightOfLight.KnightOfLight_C|GetcurrentOrbShards _asknight_of_light) 1))
  (Actor|DestroyActor))

(event EventBeginPlay
  (Physics|AddImpulse (Variables|Default|GetorbShard) (Math|Vector|MakeVector (Math|Random|RandomFloatinRange -2e+02 2e+02) (Math|Random|RandomFloatinRange -2e+02 2e+02) (Math|Random|RandomFloatinRange 6e+02 8e+02)) "None" true))

(fn ConstructionScript)

(fn ShardFloat
  (bind _orbshard (Variables|Default|GetorbShard))
  (bind _returnvalue (Transformation|GetWorldRotation _orbshard))
  (Transformation|SetWorldRotation (Variables|Default|GetorbShard) (Math|Rotator|MakeRotator (+ (.roll _returnvalue) 1.0) (+ (.pitch _returnvalue) 1.0) (+ (.yaw _returnvalue) 1.0)) false false))