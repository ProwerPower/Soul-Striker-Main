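; A switch actor that opens SwitchDoor actors when struck by a spiritOrbOG or by a KnightOfLight's AttackHitbox.
; Its Box overlap saves the orb's incoming X/Y velocity, and a hit on CubeSwitch calls the orb's non-destructible bounce.
; Opening searches all SwitchDoors for a DoorTitle matching WhichDoorToTarget and snaps their meshes to a fixed world rotation.
; Debug prints report openings and non-attack knight overlaps.
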(event OnComponentBeginOverlap(Box)
  (params (OverlappedComponent :type Primitive%20Component%20Object%20Reference) (OtherActor :type Actor%20Object%20Reference) (OtherComp :type Primitive%20Component%20Object%20Reference) (OtherBodyIndex :type Integer) (bFromSweep :type Boolean) (SweepResult :type Hit%20Result%20Structure%20%28by%20ref%29))
  (bind _asspirit_orb_og (Utilities|Casting|CastTospiritOrbOG OtherActor))
  (bind _returnvalue (Physics|GetPhysicsLinearVelocity (Variables|/Game/bluePrints/spiritOrbOG.spiritOrbOG_C|GetSphere _asspirit_orb_og) "None"))
  (Variables|/Game/bluePrints/spiritOrbOG.spiritOrbOG_C|SetOriginal%20Velocity%20X _asspirit_orb_og (.x _returnvalue))
  (Variables|/Game/bluePrints/spiritOrbOG.spiritOrbOG_C|SetOriginal%20Velocity%20Y _asspirit_orb_og (.y _returnvalue)))

(event OnComponentBeginOverlap(cubeSwitch)
  (params (OverlappedComponent :type Primitive%20Component%20Object%20Reference) (OtherActor :type Actor%20Object%20Reference) (OtherComp :type Primitive%20Component%20Object%20Reference) (OtherBodyIndex :type Integer) (bFromSweep :type Boolean) (SweepResult :type Hit%20Result%20Structure%20%28by%20ref%29))
  (bind _asknight_of_light (Utilities|Casting|CastToKnightOfLight OtherActor))
  (if (== OtherComp (Variables|/Game/ThirdPersonBP/Blueprints/KnightOfLight.KnightOfLight_C|GetattackHitbox _asknight_of_light))
    (CallFunction|OpenTargetDoor)
    (Development|PrintString "aaaaaaaaaaaaaaaaaaaaaaaaaaaaaaaaand OPEN!" true true "(R=0.018557,G=1.000000,B=0.000000,A=1.000000)" 4.0)
    (else
      (Development|PrintString "What the FUCK?" true true "(R=0.000000,G=0.660000,B=1.000000,A=1.000000)" 4.0))))

(event OnComponentHit(cubeSwitch)
  (params (HitComponent :type Primitive%20Component%20Object%20Reference) (OtherActor :type Actor%20Object%20Reference) (OtherComp :type Primitive%20Component%20Object%20Reference) (NormalImpulse :type Vector :default "0, 0, 0") (Hit :type Hit%20Result%20Structure%20%28by%20ref%29))
  (bind _asspirit_orb_og (Utilities|Casting|CastTospiritOrbOG OtherActor))
  (Default|BallBounceNon-Destructible _asspirit_orb_og)
  (CallFunction|OpenTargetDoor)
  (Development|PrintString "aaaaaaaaaaaaaaaaaaaaaaaaaaaaaaaaand OPEN!" true true "(R=0.018557,G=1.000000,B=0.000000,A=1.000000)" 4.0))

(event Custom|openTargetDoor
  (bind _outactors (Actor|GetAllActorsOfClass "/Game/bluePrints/DoorsAndDoorThings/switchDoor.switchDoor_C"))
  (for _array_element _outactors
    (if (Utilities|Enum|Equal(Enum) (Variables|/Game/bluePrints/DoorsAndDoorThings/switchDoor.switchDoor_C|GetdoorTitle _array_element) (Variables|Default|GetwhichDoorToTarget))
      (Transformation|SetWorldRotation (Variables|/Game/bluePrints/DoorsAndDoorThings/switchDoor.switchDoor_C|GetStaticMesh _array_element) "180.000000,90.000000, 0" false false))))

(fn ConstructionScript)