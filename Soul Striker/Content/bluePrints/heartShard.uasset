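; Heart shard pickup that adds one health shard to the KnightOfLight when it overlaps the shard's box, then destroys itself.
; On spawn it gets a random upward velocity impulse so it pops out with slight sideways scatter.
; If left uncollected, a hard-coded Delay chain blinks the mesh with quickening flashes as a despawn warning before destroying the actor.
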(event OnComponentBeginOverlap(Box)
  (params (OverlappedComponent :type Primitive%20Component%20Object%20Reference) (OtherActor :type Actor%20Object%20Reference) (OtherComp :type Primitive%20Component%20Object%20Reference) (OtherBodyIndex :type Integer) (bFromSweep :type Boolean) (SweepResult :type Hit%20Result%20Structure%20%28by%20ref%29))
  (bind _asknight_of_light (Utilities|Casting|CastToKnightOfLight OtherActor))
  (Variables|/Game/ThirdPersonBP/Blueprints/KnightOfLight.KnightOfLight_C|SetcurrentHealthShards _asknight_of_light (+ (Variables|/Game/ThirdPersonBP/Blueprints/KnightOfLight.KnightOfLight_C|GetcurrentHealthShards _asknight_of_light) 1))
  (Actor|DestroyActor))

(event EventBeginPlay
  (Physics|AddImpulse (Variables|Default|GetheartShard) (Math|Vector|MakeVector (Math|Random|RandomFloatinRange -2e+01 2e+01) (Math|Random|RandomFloatinRange -2e+01 2e+01) (Math|Random|RandomFloatinRange 1e+02 2e+02)) "None" true)
  (Utilities|FlowControl|Delay 5.0)
  (Rendering|SetVisibility (Variables|Default|GetheartShard) false false)
  (Utilities|FlowControl|Delay 0.1)
  (Rendering|SetVisibility (Variables|Default|GetheartShard) true false)
  (Utilities|FlowControl|Delay 1.0)
  (Rendering|SetVisibility (Variables|Default|GetheartShard) false false)
  (Utilities|FlowControl|Delay 0.1)
  (Rendering|SetVisibility (Variables|Default|GetheartShard) true false)
  (Utilities|FlowControl|Delay 1.0)
  (Rendering|SetVisibility (Variables|Default|GetheartShard) false false)
  (Utilities|FlowControl|Delay 0.1)
  (Rendering|SetVisibility (Variables|Default|GetheartShard) true false)
  (Utilities|FlowControl|Delay 1.0)
  (Rendering|SetVisibility (Variables|Default|GetheartShard) false false)
  (Utilities|FlowControl|Delay 0.1)
  (Rendering|SetVisibility (Variables|Default|GetheartShard) true false)
  (Utilities|FlowControl|Delay 0.3)
  (Rendering|SetVisibility (Variables|Default|GetheartShard) false false)
  (Utilities|FlowControl|Delay 0.1)
  (Rendering|SetVisibility (Variables|Default|GetheartShard) true false)
  (Utilities|FlowControl|Delay 0.3)
  (Rendering|SetVisibility (Variables|Default|GetheartShard) false false)
  (Utilities|FlowControl|Delay 0.1)
  (Rendering|SetVisibility (Variables|Default|GetheartShard) true false)
  (Utilities|FlowControl|Delay 0.3)
  (Rendering|SetVisibility (Variables|Default|GetheartShard) false false)
  (Utilities|FlowControl|Delay 0.1)
  (Rendering|SetVisibility (Variables|Default|GetheartShard) true false)
  (Actor|DestroyActor))

(fn ConstructionScript)