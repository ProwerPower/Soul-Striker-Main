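; Level-placed orb shard pickup that tops up the KnightOfLight's CurrentOrbShards and respawns after a cooldown.
; A looping timer runs ShardFloat, spinning the mesh and bobbing it between fixed world-Z limits by flipping the step sign.
; Box overlap by a knight holding fewer than six shards adds six, so the count can exceed six, then hides the mesh until the delay ends.
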(event OnComponentBeginOverlap(Box)
  (params (OverlappedComponent :type Primitive%20Component%20Object%20Reference) (OtherActor :type Actor%20Object%20Reference) (OtherComp :type Primitive%20Component%20Object%20Reference) (OtherBodyIndex :type Integer) (bFromSweep :type Boolean) (SweepResult :type Hit%20Result%20Structure%20%28by%20ref%29))
  (bind _asknight_of_light (Utilities|Casting|CastToKnightOfLight OtherActor))
  (if (not (Variables|Default|GetpickUpCoolDown))
    (if (< (Variables|/Game/ThirdPersonBP/Blueprints/KnightOfLight.KnightOfLight_C|GetcurrentOrbShards _asknight_of_light) 6)
      (Variables|Default|SetpickUpCoolDown true)
      (Variables|/Game/ThirdPersonBP/Blueprints/KnightOfLight.KnightOfLight_C|SetcurrentOrbShards _asknight_of_light (+ (Variables|/Game/ThirdPersonBP/Blueprints/KnightOfLight.KnightOfLight_C|GetcurrentOrbShards _asknight_of_light) 6))
      (Rendering|SetVisibility (Variables|Default|GetorbShard) false false)
      (Utilities|FlowControl|Delay 15.0)
      (Rendering|SetVisibility (Variables|Default|GetorbShard) true false)
      (Variables|Default|SetpickUpCoolDown false))))

(event EventBeginPlay
  (Utilities|Time|SetTimerbyFunctionName 0 "shardFloat" 0.1 true))

(fn ConstructionScript)

(fn ShardFloat
  (bind _orbshard (Variables|Default|GetorbShard))
  (bind _orbshard_2 (Variables|Default|GetorbShard))
  (bind _returnvalue (Transformation|GetWorldRotation _orbshard))
  (bind _returnvalue_2 (Transformation|GetWorldLocation _orbshard_2))
  (Transformation|SetWorldRotation _orbshard (Math|Rotator|MakeRotator (.roll _returnvalue) (.pitch _returnvalue) (+ (.yaw _returnvalue) 1.0)) false false)
  (if (<= (.z _returnvalue_2) (Variables|Default|GetkeyMinFloat))
    (bind _output_get (Variables|Default|SetkeyFloatMagicValue (* (Variables|Default|GetkeyFloatMagicValue) -1.0)))
    (Transformation|SetWorldLocation (Variables|Default|GetorbShard) (Math|Vector|MakeVector (.x _returnvalue_2) (.y _returnvalue_2) (+ (.z _returnvalue_2) _output_get)) false false)
    (elif (>= (.z _returnvalue_2) (Variables|Default|GetkeyMaxFloat))
      (bind _output_get_2 (Variables|Default|SetkeyFloatMagicValue (* (Variables|Default|GetkeyFloatMagicValue) -1.0)))
      (Transformation|SetWorldLocation (Variables|Default|GetorbShard) (Math|Vector|MakeVector (.x _returnvalue_2) (.y _returnvalue_2) (+ (.z _returnvalue_2) _output_get_2)) false false)
      (else
        (Transformation|SetWorldLocation (Variables|Default|GetorbShard) (Math|Vector|MakeVector (.x _returnvalue_2) (.y _returnvalue_2) (+ (.z _returnvalue_2) (Variables|Default|GetkeyFloatMagicValue))) false false)))))